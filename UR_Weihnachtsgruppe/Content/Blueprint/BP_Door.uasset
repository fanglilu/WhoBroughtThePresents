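; BP_Door is a colored delivery target that either of two players reaches to hand in a present.
; The construction script gives the mesh a dynamic material, whose doorColor parameter holds the door's color.
; On box overlap, that color is compared with the player's present color from a Material Parameter Collection.
; A match deactivates the door color, updates BP_DoorSpawner and passes its result to that player's Present success handler.
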(event OnComponentBeginOverlap(Box)
  (params (OverlappedComponent :type Primitive%20Component%20Object%20Reference) (OtherActor :type Actor%20Object%20Reference) (OtherComp :type Primitive%20Component%20Object%20Reference) (OtherBodyIndex :type Integer) (bFromSweep :type Boolean) (SweepResult :type Hit%20Result%20Structure%20%28by%20ref%29))
  (bind _dynamic (Variables|Default|Getdynamic))
  ;[1 1 1] Present Door Collision
  (bind _returnvalue (Rendering|Material|GetVectorParameterValue _dynamic "doorColor" :!class /Script/Engine.MaterialInstanceDynamic))
  (bind _output_get (Variables|Default|SetcurrentDoorColor _returnvalue))
  (Development|PrintString "Dooooor" true true _output_get 1e+02)
  (if (Utilities|ClassIsChildOf (Utilities|GetClass OtherActor) "/Game/Blueprint/BP_Character_Player_1.BP_Character_Player_1_C")
    (Variables|Default|SetisFirstPlayer true)
    (bind _returnvalue_2 (Rendering|Material|GetVectorParameterValue "/Game/Presents/presentMainColor.presentMainColor" "presentColor" :!class /Script/Engine.KismetMaterialLibrary))
    (if (== _returnvalue_2 (Variables|Default|GetcurrentDoorColor))
      (Development|PrintString "Door Color" true true (Variables|Default|GetcurrentDoorColor) 1e+02)
      (Rendering|Material|SetVectorParameterValue _dynamic "doorColor" (Variables|Default|GetdeactivatedDoorColor) :!class /Script/Engine.MaterialInstanceDynamic :!label _label)
      (bind _outactors (Actor|GetAllActorsOfClass "/Game/Blueprint/BP_DoorSpawner.BP_DoorSpawner_C"))
      (bind _updateddoorcolors (Default|UpdateDoorColors _outactors (Variables|Default|GetcurrentDoorColor)))
      (if (Variables|Default|GetisFirstPlayer)
        (bind _outactors_2 (Actor|GetAllActorsOfClass "/Game/Blueprint/Present_1.Present_1_C"))
        (Default|Player1DeliveryonSuccess _outactors_2 _updateddoorcolors)
        (else
          (bind _outactors_3 (Actor|GetAllActorsOfClass "/Game/Blueprint/Present_2.Present_2_C"))
          (Default|Player2DeliveryonSuccess _outactors_3 _updateddoorcolors))))
    (elif (Utilities|ClassIsChildOf (Utilities|GetClass OtherActor) "/Game/Blueprint/BP_Character_Player_2.BP_Character_Player_2_C")
      (Variables|Default|SetisFirstPlayer false)
      (bind _returnvalue_3 (Rendering|Material|GetVectorParameterValue "/Game/Presents/presentColor2.presentColor2" "presentColor2" :!class /Script/Engine.KismetMaterialLibrary))
      (if (== (Variables|Default|GetcurrentDoorColor) _returnvalue_3)
        (goto _label)))))

(event Collision|EventActorBeginOverlap
  (params (OtherActor :type Actor%20Object%20Reference)))

(event EventTick
  (params (DeltaSeconds :type Float%20%28single-precision%29)))

(fn ConstructionScript
  (bind _returnvalue (Rendering|Material|CreateDynamicMaterialInstance (Variables|Default|GetSM_Door) 0 "/Game/Presents/doorMaterial.doorMaterial" "None" :!class /Script/Engine.PrimitiveComponent))
  (bind _output_get (Variables|Default|Setdynamic _returnvalue))
  (Rendering|Material|SetMaterial (Variables|Default|GetSM_Door) 0 _output_get))