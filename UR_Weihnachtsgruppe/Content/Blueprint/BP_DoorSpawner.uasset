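; Spawner actor that places the colored doors at BeginPlay for the Christmas game and tracks their colors.
; Game instance difficulty picks the palette and the level name picks the transform set; colors are dealt round-robin, then shuffled for an even spread.
; Each door gets a colored dynamic material and struct, then the color list goes to Present_1.
; Helper functions remove, re-add and query remaining or unique door colors.
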(event EventBeginPlay
  (bind _gamecolors (CallFunction|ConstructColorArray))
  (Variables|Default|SetGameColors _gamecolors)
  (Variables|Default|SettotalDoors (Utilities|Array|Length (Variables|Default|GetGameTransformations)))
  (for (_array_element _array_index) (Variables|Default|GetGameTransformations)
    (Variables|Default|SetcurrentColor (Utilities|Array|Get(acopy) (Variables|Default|GetGameColors) _array_index))
    (bind _returnvalue (Game|SpawnActorfromClass "/Game/Blueprint/BP_Door.BP_Door_C" _array_element "Undefined" 0 0))
    (Variables|/Game/Blueprint/BP_Door.BP_Door_C|Setindex _returnvalue _array_index)
    (Variables|Default|SetcurrentDoor _returnvalue)
    (Rendering|Material|SetVectorParameterValue (Variables|/Game/Blueprint/BP_Door.BP_Door_C|GetdynamicMaterial _returnvalue) "doorColor" (Variables|Default|GetcurrentColor) :!class /Script/Engine.MaterialInstanceDynamic)
    (Rendering|Material|SetMaterial (Variables|/Game/Blueprint/BP_Door.BP_Door_C|GetSM_Door _returnvalue) 0 (Variables|/Game/Blueprint/BP_Door.BP_Door_C|GetdynamicMaterial _returnvalue))
    (bind _output_get (Variables|/Game/Blueprint/BP_Door.BP_Door_C|SetdoorStuct (Variables|Default|GetcurrentDoor) (Utilities|Struct|MakeS_Door (Variables|Default|GetcurrentColor) "0.000000,0.000000,0.000000" (Variables|/Game/Blueprint/BP_Door.BP_Door_C|GetSM_Door _returnvalue) 0 _array_element)))
    (Utilities|Array|Add (Variables|Default|GetMyDoorColors) (Variables|Default|GetcurrentColor))
    (Utilities|Array|Add (Variables|Default|GetMyDoors) _output_get))
  (bind _returnvalue_2 (Actor|GetActorOfClass "/Game/Blueprint/Present_1.Present_1_C"))
  (Default|AllDoorsSpawned _returnvalue_2 (Variables|Default|GetMyDoorColors)))

(fn ConstructionScript)

(fn UpdateDoorColors
  (params (colorToDelete :type Linear%20Color%20Structure))
  (bind _output_get (LocalVariables|SetlocalColorArray (Variables|Default|GetMyDoorColors)))
  (bind (_array_element _array_index) (Utilities|Array|ForEachLoopwithBreak _output_get :!label _label)
    (:LoopBody
      (bind _output_get_2 (LocalVariables|SetlocalCurrentColor _array_element))
      (bind _output_get_3 (LocalVariables|SetlocalIndex _array_index))
      (if (== _output_get_2 colorToDelete)
        (goto _label Break)))
    (:Completed
      (Utilities|Array|RemoveIndex (LocalVariables|GetlocalColorArray) _output_get_3)
      (bind _output_get_4 (Variables|Default|SetMyDoorColors (LocalVariables|GetlocalColorArray)))
      (return _output_get_4))))

(fn GetRandomColor
  (bind _colorseasy (Variables|Default|GetColorsEasy))
  (return (Utilities|Array|Get(acopy) _colorseasy (Math|Random|RandomInteger (Utilities|Array|Length _colorseasy)))))

(fn GetRemainingColors
  (return (Variables|Default|GetMyDoorColors)))

(fn AddOldtoRemaining
  (params (oldColor :type Linear%20Color%20Structure))
  (Utilities|Array|Add (Variables|Default|GetMyDoorColors) oldColor)
  (return (Variables|Default|GetMyDoorColors)))

(fn GetUniqueAvailableColors
  (for _array_element (Variables|Default|GetMyDoorColors)
    (Utilities|Array|AddUnique (LocalVariables|GetuniqueColors) _array_element))
  (return (LocalVariables|GetuniqueColors)))

(fn ConstructColorArray
  (bind _evengamecolors (LocalVariables|GetEvenGameColors))
  (bind _aschristmas_game_instance (Utilities|Casting|CastToChristmasGameInstance (Game|GetGameInstance)))
  (switch int (Variables|/Game/Blueprint/ChristmasGameInstance.ChristmasGameInstance_C|GetgameDifficulty _aschristmas_game_instance)
    (:0
      (LocalVariables|SetselectedColorLevel (Variables|Default|GetColorsEasy)))
    (:1
      (LocalVariables|SetselectedColorLevel (Variables|Default|GetColorsMedium)))
    (:2
      (LocalVariables|SetselectedColorLevel (Variables|Default|GetColorsDifficult))))
  (LocalVariables|SetmaxIndex (- (Utilities|Array|Length (LocalVariables|GetselectedColorLevel)) 1))
  (bind _returnvalue (Game|GetCurrentLevelName true))
  (if (Utilities|Enum|Equal(Enum) _returnvalue "Game_Map1_WhoBroughtThePresents")
    (Variables|Default|SetGameTransformations (Variables|Default|GetLevelTwoTransformations))
    (else
      (Variables|Default|SetGameTransformations (Variables|Default|GetLevelOneTransformations))))
  (for _array_element (Variables|Default|GetGameTransformations)
    (Utilities|Array|Add (LocalVariables|GetEvenGameColors) (Utilities|Array|Get(acopy) (LocalVariables|GetselectedColorLevel) (LocalVariables|GetcurrentIndex)))
    (if (== (LocalVariables|GetcurrentIndex) (LocalVariables|GetmaxIndex))
      (LocalVariables|SetcurrentIndex 0)
      (else
        (Math|Integer|IncrementInt (LocalVariables|GetcurrentIndex)))))
  (Utilities|Array|Shuffle _evengamecolors)
  (return _evengamecolors))