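; BP_Present_2 is the Player 2 present Blueprint, which cycles the present color as deliveries succeed.
; On BeginPlay it writes the first entry of its Colors array to the presentColor2 vector in the PresentColor2 Material Parameter Collection.
; Each Player2DeliveryOnSuccess event advances the index, wrapping at the array end, and writes the new color to the same parameter.
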(event Custom|Player%202%20Delivery%20On%20Success
  (params (delivered :type Boolean))
  (bind _colors (Variables|Default|GetColors))
  (Variables|Default|SetColor%20Index (Math|Integer|%(Integer) (+ (Variables|Default|GetColor%20Index) 1) (Utilities|Array|Length _colors)))
  (Rendering|Material|SetVectorParameterValue "/Game/Presents/presentColor2.presentColor2" "presentColor2" (Utilities|Array|Get(acopy) _colors (Variables|Default|GetColor%20Index)) :!class /Script/Engine.KismetMaterialLibrary))

(event Collision|EventActorBeginOverlap
  (params (OtherActor :type Actor%20Object%20Reference)))

(event EventTick
  (params (DeltaSeconds :type Float%20%28single-precision%29)))

(event EventBeginPlay
  (Variables|Default|SetColor%20Index 0)
  (Rendering|Material|SetVectorParameterValue "/Game/Presents/presentColor2.presentColor2" "presentColor2" (Utilities|Array|Get(acopy) (Variables|Default|GetColors) (Variables|Default|GetColor%20Index)) :!class /Script/Engine.KismetMaterialLibrary))

(fn ConstructionScript)