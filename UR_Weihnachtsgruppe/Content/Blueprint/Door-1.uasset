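; Door actor that acts as a color-matched present delivery point for two players.
; It sets its starting color in a material parameter collection on BeginPlay, using that shared value as both visual and state.
; Box overlap compares the entering player's present color with the door color, switching to a new color on a match.
; End overlap calls that player's delivery-success function on their presents without rechecking the match.
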(event OnComponentBeginOverlap(Box)
  (params (OverlappedComponent :type Primitive%20Component%20Object%20Reference) (OtherActor :type Actor%20Object%20Reference) (OtherComp :type Primitive%20Component%20Object%20Reference) (OtherBodyIndex :type Integer) (bFromSweep :type Boolean) (SweepResult :type Hit%20Result%20Structure%20%28by%20ref%29))
  ;[1 1 1] OnCollisionDetection
  (Variables|Default|SetInTheColliderBox true)
  (if (Utilities|ClassIsChildOf (Utilities|GetClass OtherActor) "/Game/Blueprint/BP_Character_Player_1.BP_Character_Player_1_C")
    (Variables|Default|SetColliderIsPlayer1 true)
    (bind _returnvalue (Rendering|Material|GetVectorParameterValue "/Game/Presents/presentMainColor.presentMainColor" "presentColor" :!class /Script/Engine.KismetMaterialLibrary))
    (bind _returnvalue_2 (Rendering|Material|GetVectorParameterValue "/Game/Presents/door_material_instance.door_material_instance" "doorColor" :!class /Script/Engine.KismetMaterialLibrary))
    (if (== _returnvalue_2 _returnvalue)
      (Rendering|Material|SetVectorParameterValue "/Game/Presents/door_material_instance.door_material_instance" "doorColor" (Variables|Default|GetnewDoorColor) :!class /Script/Engine.KismetMaterialLibrary :!label _label))
    (elif (Utilities|ClassIsChildOf (Utilities|GetClass OtherActor) "/Game/Blueprint/BP_Character_Player_2.BP_Character_Player_2_C")
      (Variables|Default|SetColliderIsPlayer2 true)
      (bind _returnvalue_3 (Rendering|Material|GetVectorParameterValue "/Game/Presents/presentColor2.presentColor2" "presentColor2" :!class /Script/Engine.KismetMaterialLibrary))
      (bind _returnvalue_4 (Rendering|Material|GetVectorParameterValue "/Game/Presents/door_material_instance.door_material_instance" "doorColor" :!class /Script/Engine.KismetMaterialLibrary))
      (if (== _returnvalue_4 _returnvalue_3)
        (goto _label)))))

(event OnComponentEndOverlap(Box)
  (params (OverlappedComponent :type Primitive%20Component%20Object%20Reference) (OtherActor :type Actor%20Object%20Reference) (OtherComp :type Primitive%20Component%20Object%20Reference) (OtherBodyIndex :type Integer))
  ;[1 1 1] OnCollisionDetection
  (if (Utilities|ClassIsChildOf (Utilities|GetClass OtherActor) "/Game/Blueprint/BP_Character_Player_1.BP_Character_Player_1_C")
    (bind _outactors (Actor|GetAllActorsOfClass "/Game/Blueprint/Present_1.Present_1_C"))
    (Default|Player1DeliveryonSuccess _outactors true)
    (elif (Utilities|ClassIsChildOf (Utilities|GetClass OtherActor) "/Game/Blueprint/BP_Character_Player_2.BP_Character_Player_2_C")
      (bind _outactors_2 (Actor|GetAllActorsOfClass "/Game/Blueprint/BP_Present_2.BP_Present_2_C"))
      (Default|Player2DeliveryonSuccess _outactors_2 false))))

(event EventBeginPlay
  (Rendering|Material|SetVectorParameterValue "/Game/Presents/door_material_instance.door_material_instance" "doorColor" (Variables|Default|GetinitialColor) :!class /Script/Engine.KismetMaterialLibrary))

(fn ConstructionScript)