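; Light pole pickup for two players that gives the user light mode or inflicts dark mode on the opponent.
; Box overlap shows a per-player prompt widget, with tutorial-map variants.
; ActivateLightPole picks the effect via DamageOther, starts a timer on Player 1's character for either player, sets the mode flag and fires a lightpost update dispatcher.
; It then spawns a replacement at a random map-specific transform, plays a sound and destroys itself.
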(event OnComponentEndOverlap(Box)
  (params (OverlappedComponent :type Primitive%20Component%20Object%20Reference) (OtherActor :type Actor%20Object%20Reference) (OtherComp :type Primitive%20Component%20Object%20Reference) (OtherBodyIndex :type Integer))
  ;[1 1 1] OnCollisionDetection
  (Variables|Default|SetInTheColliderBox false)
  (if (Variables|Default|GetColliderIsPlayer1)
    (Widget|RemovefromParent (stale OnComponentBeginOverlap(Box) _returnvalue_3))
    (Variables|Default|SetColliderIsPlayer1 false)
    (Variables|Default|SetWidgetIsActive_Player1 false)
    (elif (Variables|Default|GetColliderIsPlayer2)
      (Widget|RemovefromParent (stale OnComponentBeginOverlap(Box) _returnvalue_6))
      (Variables|Default|SetColliderIsPlayer2 false)
      (Variables|Default|SetWidgetIsActive_Player2 false))))

(event OnComponentBeginOverlap(Box)
  (params (OverlappedComponent :type Primitive%20Component%20Object%20Reference) (OtherActor :type Actor%20Object%20Reference) (OtherComp :type Primitive%20Component%20Object%20Reference) (OtherBodyIndex :type Integer) (bFromSweep :type Boolean) (SweepResult :type Hit%20Result%20Structure%20%28by%20ref%29))
  ;[1 1 1] OnCollisionDetection
  (Variables|Default|SetInTheColliderBox true)
  (if (Utilities|ClassIsChildOf (Utilities|GetClass OtherActor) "/Game/Blueprint/BP_Character_Player_1.BP_Character_Player_1_C")
    (Variables|Default|SetColliderIsPlayer1 true)
    (if (not (Variables|Default|GetWidgetIsActive_Player1))
      (Variables|Default|SetWidgetIsActive_Player1 true)
      (bind _returnvalue (Game|GetCurrentLevelName true))
      (if (Utilities|Enum|Equal(Enum) _returnvalue "Game_Map_WhoBroughtThePresents_Tutorial")
        (bind _returnvalue_2 (UserInterface|CreateWidget "/Game/Blueprint/TutorialWidgets/Tutorial/TUTORIAL_BP_GameWidget_LightItem_Player1_2.TUTORIAL_BP_GameWidget_LightItem_Player1_2_C"))
        (UserInterface|Viewport|AddtoViewport _returnvalue_2 0)
        (else
          (bind _returnvalue_3 (UserInterface|CreateWidget "/Game/Blueprint/UI_Widget/BP_GameWidget_LightItem_Player1.BP_GameWidget_LightItem_Player1_C"))
          (UserInterface|Viewport|AddtoViewport _returnvalue_3 0))))
    (elif (Utilities|ClassIsChildOf (Utilities|GetClass OtherActor) "/Game/Blueprint/BP_Character_Player_2.BP_Character_Player_2_C")
      (Variables|Default|SetColliderIsPlayer2 true)
      (if (not (Variables|Default|GetWidgetIsActive_Player2))
        (Variables|Default|SetWidgetIsActive_Player2 true)
        (bind _returnvalue_4 (Game|GetCurrentLevelName true))
        (if (Utilities|Enum|Equal(Enum) _returnvalue_4 "Game_Map_WhoBroughtThePresents_Tutorial")
          (bind _returnvalue_5 (UserInterface|CreateWidget "/Game/Blueprint/TutorialWidgets/Tutorial/TUTORIAL_BP_GameWidget_LightItem_Player2_2.TUTORIAL_BP_GameWidget_LightItem_Player2_2_C"))
          (UserInterface|Viewport|AddtoViewport _returnvalue_5 0)
          (else
            (bind _returnvalue_6 (UserInterface|CreateWidget "/Game/Blueprint/UI_Widget/BP_GameWidget_LightItem_Player2.BP_GameWidget_LightItem_Player2_C"))
            (UserInterface|Viewport|AddtoViewport _returnvalue_6 0)))))))

(event Custom|SwitchLightMode_Player2
  (params (On :type Boolean))
  (bind _returnvalue (Actor|GetActorOfClass "/Game/Blueprint/BP_Character_Player_2.BP_Character_Player_2_C"))
  (if On
    (Variables|/Game/Blueprint/BP_Character_Player_2.BP_Character_Player_2_C|SetisLightModeOn _returnvalue true)
    (else
      (Variables|/Game/Blueprint/BP_Character_Player_2.BP_Character_Player_2_C|SetisLightModeOn _returnvalue false)))
  (Default|CallLightpostUpdatePlayer2EventDispatcher))

(event Custom|ActivateLightPole
  (params (DamageOther :type Boolean))
  (if DamageOther
    (if (and (Variables|Default|GetInTheColliderBox) (Variables|Default|GetColliderIsPlayer1))
      (bind _returnvalue (Actor|GetActorOfClass "/Game/Blueprint/BP_Character_Player_1.BP_Character_Player_1_C"))
      (Default|TriggerTimer _returnvalue true false false true)
      (CallFunction|SwitchDarkModePlayer2 true)
      (if (Variables|Default|GetWidgetIsActive_Player1) :!label _label
        (Widget|RemovefromParent (stale OnComponentBeginOverlap(Box) _returnvalue_3))
        (Variables|Default|SetWidgetIsActive_Player1 false)
        (bind _returnvalue_2 (Game|GetCurrentLevelName true :!label _label_2))
        (if (Utilities|Enum|Equal(Enum) _returnvalue_2 "Game_Map_WhoBroughtThePresents_Tutorial")
          (Game|SpawnActorfromClass "ItemCollision_LightPole_C" (Utilities|Array|Get(acopy) (Variables|Default|GetTransformArray_TUTORIAL) (Math|Random|RandomIntegerinRange 0 (- (Utilities|Array|Length (Variables|Default|GetTransformArray_TUTORIAL)) 1))) "Undefined" 0 0)
          (else
            (Game|SpawnActorfromClass "ItemCollision_LightPole_C" (Utilities|Array|Get(acopy) (Variables|Default|GetTransformArray) (Math|Random|RandomIntegerinRange 0 (- (Utilities|Array|Length (Variables|Default|GetTransformArray)) 1))) "Undefined" 0 0)))
        (if DamageOther
          (Audio|PlaySound2D "/Game/Music/SoundEffects/mixkit-wrong-answer-fail-notification-946.mixkit-wrong-answer-fail-notification-946" 1.0 1.0 0.0 0 0)
          (else
            (Audio|PlaySound2D "/Game/Music/SoundEffects/mixkit-positive-notification-951.mixkit-positive-notification-951" 1.0 1.0 0.0 0 0)))
        (Actor|DestroyActor)
        (elif (Variables|Default|GetWidgetIsActive_Player2)
          (Widget|RemovefromParent (stale OnComponentBeginOverlap(Box) _returnvalue_6))
          (Variables|Default|SetWidgetIsActive_Player2 false)
          (goto _label_2)))
      (elif (and (Variables|Default|GetInTheColliderBox) (Variables|Default|GetColliderIsPlayer2))
        (bind _returnvalue_3 (Actor|GetActorOfClass "/Game/Blueprint/BP_Character_Player_1.BP_Character_Player_1_C"))
        (Default|TriggerTimer _returnvalue_3 false false false true)
        (CallFunction|SwitchDarkModePlayer1 true)
        (goto _label)))
    (elif (and (Variables|Default|GetInTheColliderBox) (Variables|Default|GetColliderIsPlayer1))
      (bind _returnvalue_4 (Actor|GetActorOfClass "/Game/Blueprint/BP_Character_Player_1.BP_Character_Player_1_C"))
      (Default|TriggerTimer _returnvalue_4 true false false true)
      (CallFunction|SwitchLightModePlayer1 true)
      (goto _label)
      (elif (and (Variables|Default|GetInTheColliderBox) (Variables|Default|GetColliderIsPlayer2))
        (bind _returnvalue_5 (Actor|GetActorOfClass "/Game/Blueprint/BP_Character_Player_1.BP_Character_Player_1_C"))
        (Default|TriggerTimer _returnvalue_5 false false false true)
        (CallFunction|SwitchLightModePlayer2 true)
        (goto _label)))))

(event Custom|SwitchLightMode_Player1
  (params (On :type Boolean))
  (bind _returnvalue (Actor|GetActorOfClass "/Game/Blueprint/BP_Character_Player_1.BP_Character_Player_1_C"))
  (if On
    (Variables|/Game/Blueprint/BP_Character_Player_1.BP_Character_Player_1_C|SetisLightModeOn _returnvalue true)
    (else
      (Variables|/Game/Blueprint/BP_Character_Player_1.BP_Character_Player_1_C|SetisLightModeOn _returnvalue false)))
  (Default|CallLightpostUpdatePlayer1EventDispatcher))

(event Custom|SwitchDarkMode_Player1
  (params (On :type Boolean))
  (bind _returnvalue (Actor|GetActorOfClass "/Game/Blueprint/BP_Character_Player_1.BP_Character_Player_1_C"))
  (if On
    (Variables|/Game/Blueprint/BP_Character_Player_1.BP_Character_Player_1_C|SetisDarkModeOn _returnvalue true)
    (else
      (Variables|/Game/Blueprint/BP_Character_Player_1.BP_Character_Player_1_C|SetisDarkModeOn _returnvalue false)))
  (Default|CallLightpostUpdatePlayer1EventDispatcher))

(event Custom|SwitchDarkMode_Player2
  (params (On :type Boolean))
  (bind _returnvalue (Actor|GetActorOfClass "/Game/Blueprint/BP_Character_Player_2.BP_Character_Player_2_C"))
  (if On
    (Variables|/Game/Blueprint/BP_Character_Player_2.BP_Character_Player_2_C|SetisDarkModeOn _returnvalue true)
    (else
      (Variables|/Game/Blueprint/BP_Character_Player_2.BP_Character_Player_2_C|SetisDarkModeOn _returnvalue false)))
  (Default|CallLightpostUpdatePlayer2EventDispatcher))

(fn ConstructionScript)