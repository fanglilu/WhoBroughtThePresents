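; Teleport pickup that sends Player 1 or 2 to the BP_Door matching their current present color.
; On overlap it reads that player's color from a parameter collection, finds the matching door material, then after a delay moves the player in front of it with yaw flipped.
; The item's mesh follows, sinks on a timeline, then respawns at the next point in a cyclic, level-specific location list, with overlaps gated until then.
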(event OnComponentBeginOverlap(Box)
  (params (OverlappedComponent :type Primitive%20Component%20Object%20Reference) (OtherActor :type Actor%20Object%20Reference) (OtherComp :type Primitive%20Component%20Object%20Reference) (OtherBodyIndex :type Integer) (bFromSweep :type Boolean) (SweepResult :type Hit%20Result%20Structure%20%28by%20ref%29))
  (bind _returnvalue (Utilities|GetClass OtherActor))
  (bind _staticmesh (Variables|Default|GetStaticMesh))
  (bind _returnvalue_2 (Transformation|GetWorldLocation _staticmesh))
  (bind (_x _y _z) (Math|Vector|BreakVector _returnvalue_2))
  (bind _outactors (Actor|GetAllActorsOfClass "/Game/Blueprint/BP_Door.BP_Door_C"))
  (Variables|Default|SetAllDoors _outactors)
  (if (Variables|Default|GetallowOverlap)
    (if (Utilities|ClassIsChildOf _returnvalue "/Game/Blueprint/BP_Character_Player_1.BP_Character_Player_1_C")
      (bind _returnvalue_3 (Actor|GetActorOfClass "/Game/Blueprint/BP_Character_Player_1.BP_Character_Player_1_C"))
      (Variables|Default|Setplayer _returnvalue_3)
      (bind _returnvalue_4 (Rendering|Material|GetVectorParameterValue "/Game/Presents/presentMainColor.presentMainColor" "presentColor" :!class /Script/Engine.KismetMaterialLibrary))
      (Variables|Default|SetpresentColor _returnvalue_4)
      (Variables|Default|SetallowOverlap false :!label _label)
      (bind _array_element (Utilities|Array|ForEachLoopwithBreak (Variables|Default|GetAllDoors) :!label _label_2)
        (:LoopBody
          (bind _returnvalue_5 (Rendering|Material|GetVectorParameterValue (Variables|/Game/Blueprint/BP_Door.BP_Door_C|GetdynamicMaterial _array_element) "doorColor" :!class /Script/Engine.MaterialInstanceDynamic))
          (if (== _returnvalue_5 (Variables|Default|GetpresentColor))
            (Variables|Default|SetTargetDoor _array_element)
            (goto _label_2 Break)))
        (:Completed
          (Utilities|FlowControl|Delay 1.0)
          (Transformation|SetActorLocationAndRotation (Variables|Default|Getplayer) (+ (Transformation|GetWorldLocation (Variables|/Game/Blueprint/BP_Door.BP_Door_C|GetSM_Door (Variables|Default|GetTargetDoor))) (* (Math|Vector|GetForwardVector (Variables|/Game/Blueprint/BP_Door.BP_Door_C|GetSM_Door (Variables|Default|GetTargetDoor))) 3e+02)) (Transformation|GetWorldRotation (Variables|/Game/Blueprint/BP_Door.BP_Door_C|GetSM_Door (Variables|Default|GetTargetDoor))) false true)
          (Pawn|SetControlRotation (Pawn|GetController (Variables|Default|Getplayer)) (Math|Rotator|MakeRotator (.Roll (Math|Rotator|BreakRotator (Transformation|GetWorldRotation (Variables|/Game/Blueprint/BP_Door.BP_Door_C|GetSM_Door (Variables|Default|GetTargetDoor))))) (.Pitch (Math|Rotator|BreakRotator (Transformation|GetWorldRotation (Variables|/Game/Blueprint/BP_Door.BP_Door_C|GetSM_Door (Variables|Default|GetTargetDoor))))) (+ (.Yaw (Math|Rotator|BreakRotator (Transformation|GetWorldRotation (Variables|/Game/Blueprint/BP_Door.BP_Door_C|GetSM_Door (Variables|Default|GetTargetDoor))))) 1.8e+02)))
          (Transformation|SetWorldLocation (Variables|Default|GetStaticMesh) (+ (Transformation|GetWorldLocation (Variables|/Game/Blueprint/BP_Door.BP_Door_C|GetSM_Door (Variables|Default|GetTargetDoor))) (* (Math|Vector|GetForwardVector (Variables|/Game/Blueprint/BP_Door.BP_Door_C|GetSM_Door (Variables|Default|GetTargetDoor))) 3e+02)) false false)
          (bind _timer (Timeline|Timeline PlayFromStart)
            (:Update
              (Transformation|SetWorldLocation (Variables|Default|GetStaticMesh) (Math|Vector|MakeVector _x _y (Math|Float|Lerp _z -1e+02 _timer)) false true))
            (:Finished
              (CallFunction|SpawnTeleportItemtoNewLocation)
              (Variables|Default|SetallowOverlap true)
              (Timeline|Timeline Stop)))))
      (elif (Utilities|ClassIsChildOf _returnvalue "/Game/Blueprint/BP_Character_Player_2.BP_Character_Player_2_C")
        (bind _returnvalue_6 (Actor|GetActorOfClass "/Game/Blueprint/BP_Character_Player_2.BP_Character_Player_2_C"))
        (Variables|Default|Setplayer _returnvalue_6)
        (bind _returnvalue_7 (Rendering|Material|GetVectorParameterValue "/Game/Presents/presentColor2.presentColor2" "presentColor2" :!class /Script/Engine.KismetMaterialLibrary))
        (Variables|Default|SetpresentColor _returnvalue_7)
        (goto _label)))))

(event EventBeginPlay)

(event Collision|EventActorBeginOverlap
  (params (OtherActor :type Actor%20Object%20Reference)))

(event EventTick
  (params (DeltaSeconds :type Float%20%28single-precision%29)))

(fn ConstructionScript)

(fn SpawnTeleportItemtoNewLocation
  (bind _returnvalue (Game|GetCurrentLevelName true))
  (if (Utilities|Enum|Equal(Enum) _returnvalue "Game_Map1_WhoBroughtThePresents")
    (bind _result (Math|Integer|DecrementInt (Utilities|Array|Length (Variables|Default|GetspawingLocations_Level2)))
      (:%20%20
        (if (== _result (Variables|Default|GetlocaionIndex))
          (Variables|Default|SetlocaionIndex 0)
          (else
            (Math|Integer|IncrementInt (Variables|Default|GetlocaionIndex)
              (:%20%20
                _))))
        (Transformation|SetWorldLocation (Variables|Default|GetStaticMesh) (Utilities|Array|Get(acopy) (Variables|Default|GetspawingLocations_Level2) (Variables|Default|GetlocaionIndex)) false true)))
    (else
      (bind _result_2 (Math|Integer|DecrementInt (Utilities|Array|Length (Variables|Default|GetspawingLocations)))
        (:%20%20
          (if (== _result_2 (Variables|Default|GetlocaionIndex))
            (Variables|Default|SetlocaionIndex 0)
            (else
              (Math|Integer|IncrementInt (Variables|Default|GetlocaionIndex)
                (:%20%20
                  _))))
          (Transformation|SetWorldLocation (Variables|Default|GetStaticMesh) (Utilities|Array|Get(acopy) (Variables|Default|GetspawingLocations) (Variables|Default|GetlocaionIndex)) false true))))))