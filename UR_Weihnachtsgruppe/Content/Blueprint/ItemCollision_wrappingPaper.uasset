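; Wrapping paper item actor that shows a player-specific widget when Player 1 or Player 2 enters its collision box.
; Begin overlap checks the other actor's class, sets that player's flag and adds the matching widget to the viewport.
; End overlap uses the stored flags rather than the leaving actor to remove the widget, then destroys the item.
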(event OnComponentBeginOverlap(Box)
  (params (OverlappedComponent :type Primitive%20Component%20Object%20Reference) (OtherActor :type Actor%20Object%20Reference) (OtherComp :type Primitive%20Component%20Object%20Reference) (OtherBodyIndex :type Integer) (bFromSweep :type Boolean) (SweepResult :type Hit%20Result%20Structure%20%28by%20ref%29))
  ;[1 1 1] OnCollisionDetection
  (Variables|Default|SetInTheColliderBox true)
  (if (Utilities|ClassIsChildOf (Utilities|GetClass OtherActor) "/Game/Blueprint/BP_Character_Player_1.BP_Character_Player_1_C")
    (Variables|Default|SetColliderIsPlayer1 true)
    (bind _returnvalue (UserInterface|CreateWidget "/Game/Blueprint/UI_Widget/BP_GameWidget_WrappingPaperItem_Player1.BP_GameWidget_WrappingPaperItem_Player1_C"))
    (UserInterface|Viewport|AddtoViewport _returnvalue 0)
    (elif (Utilities|ClassIsChildOf (Utilities|GetClass OtherActor) "/Game/Blueprint/BP_Character_Player_2.BP_Character_Player_2_C")
      (Variables|Default|SetColliderIsPlayer2 true)
      (bind _returnvalue_2 (UserInterface|CreateWidget "/Game/Blueprint/UI_Widget/BP_GameWidget_WrappingPaperItem_Player2_.BP_GameWidget_WrappingPaperItem_Player2__C"))
      (UserInterface|Viewport|AddtoViewport _returnvalue_2 0))))

(event OnComponentEndOverlap(Box)
  (params (OverlappedComponent :type Primitive%20Component%20Object%20Reference) (OtherActor :type Actor%20Object%20Reference) (OtherComp :type Primitive%20Component%20Object%20Reference) (OtherBodyIndex :type Integer))
  ;[1 1 1] OnCollisionDetection
  (Variables|Default|SetInTheColliderBox false)
  (if (Variables|Default|GetColliderIsPlayer1)
    (Widget|RemovefromParent (stale OnComponentBeginOverlap(Box) _returnvalue))
    (Variables|Default|SetColliderIsPlayer1 false)
    (Actor|DestroyActor)
    (elif (Variables|Default|GetColliderIsPlayer2)
      (Widget|RemovefromParent (stale OnComponentBeginOverlap(Box) _returnvalue_2))
      (Variables|Default|SetColliderIsPlayer2 false)
      (Actor|DestroyActor))))

(fn ConstructionScript)