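; Light post actor whose point light reacts to nearby players in dark mode.
; Entering its detection box toggles the light if that player's IsDarkModeOn is set, otherwise restores the visibility saved at BeginPlay; leaving restores it only while dark mode is on.
; GetAllowToggle reads the flag from the first actor found of the matching Player 1 or 2 class.
; The T key flips Player 1's dark mode and prints a debug string.
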(event OnComponentBeginOverlap(BoxNearDetect)
  (params (OverlappedComponent :type Primitive%20Component%20Object%20Reference) (OtherActor :type Actor%20Object%20Reference) (OtherComp :type Primitive%20Component%20Object%20Reference) (OtherBodyIndex :type Integer) (bFromSweep :type Boolean) (SweepResult :type Hit%20Result%20Structure%20%28by%20ref%29))
  (bind _pointlight (Variables|Default|GetPointLight))
  ;[1 1 1] Toggle Light (false) when dark mode is on for player
  (bind _allowtoggle (CallFunction|GetAllowToggle OtherActor))
  (if _allowtoggle
    (Rendering|ToggleVisibility _pointlight false)
    (else
      (Rendering|SetVisibility _pointlight (Variables|Default|GetinitialState) false))))

(event OnComponentEndOverlap(BoxNearDetect)
  (params (OverlappedComponent :type Primitive%20Component%20Object%20Reference) (OtherActor :type Actor%20Object%20Reference) (OtherComp :type Primitive%20Component%20Object%20Reference) (OtherBodyIndex :type Integer))
  ;[1 1 1] Reset To Initial State When Overlap End
  (bind _allowtoggle (CallFunction|GetAllowToggle OtherActor))
  (if _allowtoggle
    (Rendering|SetVisibility (Variables|Default|GetPointLight) (Variables|Default|GetinitialState) false)))

(event EventBeginPlay
  ;[1 1 1] Initialize Visibilty (true)
  (Variables|Default|SetinitialState (Variables|/Script/Engine.SceneComponent|GetbVisible (Variables|Default|GetPointLight)))
  (Input|EnableInput (Game|GetPlayerController 0)))

(event Input|KeyboardEvents|T
  (params (Key :type Key%20Structure :default "None"))
  ;[1 1 1] For Yara - Toggle dark mode of player 1
  (:Pressed
    (Development|PrintString "Event T")
    (bind _returnvalue (Actor|GetActorOfClass "/Game/Blueprint/BP_Character_Player_1.BP_Character_Player_1_C"))
    (if (Variables|/Game/Blueprint/BP_Character_Player_1.BP_Character_Player_1_C|GetisDarkModeOn _returnvalue)
      (Variables|/Game/Blueprint/BP_Character_Player_1.BP_Character_Player_1_C|SetisDarkModeOn _returnvalue false)
      (else
        (Variables|/Game/Blueprint/BP_Character_Player_1.BP_Character_Player_1_C|SetisDarkModeOn _returnvalue true)))))

(fn ConstructionScript)

(fn GetAllowToggle
  (params (player :type Actor%20Object%20Reference))
  (bind _returnvalue (Utilities|GetClass player))
  (if (Utilities|ClassIsChildOf _returnvalue "/Game/Blueprint/BP_Character_Player_1.BP_Character_Player_1_C")
    (bind _returnvalue_2 (Actor|GetActorOfClass "/Game/Blueprint/BP_Character_Player_1.BP_Character_Player_1_C"))
    (return (Variables|/Game/Blueprint/BP_Character_Player_1.BP_Character_Player_1_C|GetisDarkModeOn _returnvalue_2))
    (elif (Utilities|ClassIsChildOf _returnvalue "/Game/Blueprint/BP_Character_Player_2.BP_Character_Player_2_C")
      (bind _returnvalue_3 (Actor|GetActorOfClass "/Game/Blueprint/BP_Character_Player_2.BP_Character_Player_2_C"))
      (return (Variables|/Game/Blueprint/BP_Character_Player_2.BP_Character_Player_2_C|GetisDarkModeOn _returnvalue_3)))))