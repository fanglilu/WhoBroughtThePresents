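; LightPostOff is a light post whose point light flips visibility when a player character with light mode on comes near.
; BeginPlay stores the light's initial visibility.
; BoxNearDetect overlaps toggle the light if allowed or restore that state otherwise, and exiting restores it only if still allowed.
; GetAllowToggle matches the actor to either player class, then reads IsLightModeOn via GetActorOfClass rather than from the overlapping actor.
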(event OnComponentBeginOverlap(BoxNearDetect)
  (params (OverlappedComponent :type Primitive%20Component%20Object%20Reference) (OtherActor :type Actor%20Object%20Reference) (OtherComp :type Primitive%20Component%20Object%20Reference) (OtherBodyIndex :type Integer) (bFromSweep :type Boolean) (SweepResult :type Hit%20Result%20Structure%20%28by%20ref%29))
  (bind _pointlight (Variables|Default|GetPointLight))
  ;[1 1 1] Toggle Light (true) when Light Mode for player is On
  (bind _allowtoggle (CallFunction|GetAllowToggle OtherActor))
  (if _allowtoggle
    (Rendering|ToggleVisibility _pointlight false)
    (else
      (Rendering|SetVisibility _pointlight (Variables|Default|GetinitialState) false))))

(event OnComponentEndOverlap(BoxNearDetect)
  (params (OverlappedComponent :type Primitive%20Component%20Object%20Reference) (OtherActor :type Actor%20Object%20Reference) (OtherComp :type Primitive%20Component%20Object%20Reference) (OtherBodyIndex :type Integer))
  ;[1 1 1] Comment
  (bind _allowtoggle (CallFunction|GetAllowToggle OtherActor))
  (if _allowtoggle
    (Rendering|SetVisibility (Variables|Default|GetPointLight) (Variables|Default|GetinitialState) false)))

(event EventBeginPlay
  ;[1 1 1] Initialize Visibility (false)
  (Variables|Default|SetinitialState (Variables|/Script/Engine.SceneComponent|GetbVisible (Variables|Default|GetPointLight))))

(fn ConstructionScript)

(fn GetAllowToggle
  (params (player :type Actor%20Object%20Reference))
  (bind _returnvalue (Utilities|GetClass player))
  (if (Utilities|ClassIsChildOf _returnvalue "/Game/Blueprint/BP_Character_Player_1.BP_Character_Player_1_C")
    (bind _returnvalue_2 (Actor|GetActorOfClass "/Game/Blueprint/BP_Character_Player_1.BP_Character_Player_1_C"))
    (return (Variables|/Game/Blueprint/BP_Character_Player_1.BP_Character_Player_1_C|GetisLightModeOn _returnvalue_2))
    (elif (Utilities|ClassIsChildOf _returnvalue "/Game/Blueprint/BP_Character_Player_2.BP_Character_Player_2_C")
      (bind _returnvalue_3 (Actor|GetActorOfClass "/Game/Blueprint/BP_Character_Player_2.BP_Character_Player_2_C"))
      (return (Variables|/Game/Blueprint/BP_Character_Player_2.BP_Character_Player_2_C|GetisLightModeOn _returnvalue_3)))))