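; A static light post actor with a point light whose visibility is set from LightpostVisible at BeginPlay.
; GetAllowToggle checks whether the given player is a Player 1 or Player 2 character class and returns that character's IsLightModeOn flag.
; It fetches the character through GetActorOfClass rather than reading the passed-in reference.
; The toggle itself is not implemented in this Blueprint.
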(event EventBeginPlay
  ;[1 1 1] Initialize Visibility
  (Rendering|SetVisibility (Variables|Default|GetPointLight) (Variables|Default|GetLightpostVisible) false))

(fn ConstructionScript)

(fn GetAllowToggle
  (params (player :type Actor%20Object%20Reference))
  (bind _returnvalue (Utilities|GetClass player))
  (if (Utilities|ClassIsChildOf _returnvalue "/Game/Blueprint/BP_Character_Player_1.BP_Character_Player_1_C")
    (bind _returnvalue_2 (Actor|GetActorOfClass "/Game/Blueprint/BP_Character_Player_1.BP_Character_Player_1_C"))
    (return (Variables|/Game/Blueprint/BP_Character_Player_1.BP_Character_Player_1_C|GetisLightModeOn _returnvalue_2))
    (elif (Utilities|ClassIsChildOf _returnvalue "/Game/Blueprint/BP_Character_Player_2.BP_Character_Player_2_C")
      (bind _returnvalue_3 (Actor|GetActorOfClass "/Game/Blueprint/BP_Character_Player_2.BP_Character_Player_2_C"))
      (return (Variables|/Game/Blueprint/BP_Character_Player_2.BP_Character_Player_2_C|GetisLightModeOn _returnvalue_3)))))