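; MagicItemColorSwticher cycles the magicColor parameter of the MagicEffect Material Parameter Collection through the game's color palette.
; Tick feeds a 0.2-second Delay, which throttles the color changes to that interval.
; Each step looks up BP_DoorSpawner, writes its GameColors entry at ColorIndex to the collection, then advances the index, wrapping to zero after the last color.
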(event EventBeginPlay)

(event Collision|EventActorBeginOverlap
  (params (OtherActor :type Actor%20Object%20Reference)))

(event EventTick
  (params (DeltaSeconds :type Float%20%28single-precision%29))
  (Utilities|FlowControl|Delay 0.2)
  (bind _returnvalue (Actor|GetActorOfClass "/Game/Blueprint/BP_DoorSpawner.BP_DoorSpawner_C"))
  (Rendering|Material|SetVectorParameterValue "/Game/Presents/magicEffect.magicEffect" "magicColor" (Utilities|Array|Get(acopy) (Variables|/Game/Blueprint/BP_DoorSpawner.BP_DoorSpawner_C|GetGameColors _returnvalue) (Variables|Default|GetcolorIndex)) :!class /Script/Engine.KismetMaterialLibrary)
  (bind _result (Math|Integer|DecrementInt (Utilities|Array|Length (Variables|/Game/Blueprint/BP_DoorSpawner.BP_DoorSpawner_C|GetGameColors _returnvalue)))
    (:%20%20
      (if (== _result (Variables|Default|GetColorIndex))
        (Variables|Default|SetColorIndex 0)
        (else
          (Math|Integer|IncrementInt (Variables|Default|GetColorIndex)))))))

(fn ConstructionScript)