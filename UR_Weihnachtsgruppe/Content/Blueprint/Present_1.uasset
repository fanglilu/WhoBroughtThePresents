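; Player 1's present Blueprint, which assigns and changes the color of the present to deliver, drawn from BP_DoorSpawner's door colors.
; Once all doors spawn it randomly picks colors for both presents, and a successful Player 1 delivery rerolls its own.
; When allowed, shuffling cycles through unique available colors and hands the old one back to the spawner.
; Colors live in Material Parameter Collections, with the spawner updated after each pick.
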(event Custom|Player%201%20Delivery%20On%20Success
  (params (availableDoorColors :type Array%20of%20Linear%20Color%20Structures))
  (bind _newcolor (CallFunction|SetRandomPresentColor availableDoorColors))
  (bind _returnvalue (Actor|GetActorOfClass "/Game/Blueprint/BP_DoorSpawner.BP_DoorSpawner_C"))
  (Default|UpdateDoorColors _returnvalue _newcolor))

(event Custom|All%20Doors%20Spawned
  (params (available%20Colors :type Array%20of%20Linear%20Color%20Structures))
  (bind _newcolor (CallFunction|SetRandomPresentColor available%20Colors))
  (bind _outactors (Actor|GetAllActorsOfClass "/Game/Blueprint/BP_DoorSpawner.BP_DoorSpawner_C"))
  (bind _updateddoorcolors (Default|UpdateDoorColors _outactors _newcolor))
  (bind _output_get (Variables|Default|Setpresent2%20color (Utilities|Array|Get(acopy) _updateddoorcolors (Math|Random|RandomInteger (Utilities|Array|Length _updateddoorcolors)))))
  (Rendering|Material|SetVectorParameterValue "/Game/Presents/presentColor2.presentColor2" "presentColor2" _output_get :!class /Script/Engine.KismetMaterialLibrary)
  (bind _returnvalue (Actor|GetActorOfClass "/Game/Blueprint/BP_DoorSpawner.BP_DoorSpawner_C"))
  (bind _updateddoorcolors_2 (Default|UpdateDoorColors _returnvalue _output_get))
  (for _array_element _updateddoorcolors_2
    (Development|PrintString "After Santa Color" true true _array_element 1e+02)))

(event Custom|Present%201%20On%20Color%20Shuffle
  (if (Variables|Default|GetallowChange)
    (bind _returnvalue (Actor|GetActorOfClass "/Game/Blueprint/BP_DoorSpawner.BP_DoorSpawner_C"))
    (bind _output_get (Variables|Default|Setdoor%20spawner _returnvalue))
    (bind _shufflecolors (Default|GetUniqueAvailableColors _output_get))
    (Variables|Default|SetuniqueColors _shufflecolors)
    (Variables|Default|SetmaxIndex (- (Utilities|Array|Length _shufflecolors) 1))
    (Development|PrintString (Utilities|String|ToString(Boolean) (<= (Variables|Default|GetshuffleIndex) (Variables|Default|GetmaxIndex))))
    (if (<= (Variables|Default|GetshuffleIndex) (Variables|Default|GetmaxIndex))
      (bind _output_get_2 (Variables|Default|SetnewColor (Utilities|Array|Get(acopy) (Variables|Default|GetuniqueColors) (Variables|Default|GetshuffleIndex))))
      (CallFunction|SwitchColors _output_get_2)
      (else
        (bind _output_get_3 (Variables|Default|SetshuffleIndex 0))
        (bind _output_get_4 (Variables|Default|SetnewColor (Utilities|Array|Get(acopy) (Variables|Default|GetuniqueColors) _output_get_3)))
        (CallFunction|SwitchColors _output_get_4)))
    (Default|UpdateDoorColors (Variables|Default|Getdoor%20spawner) (Variables|Default|GetnewColor))
    (Variables|Default|SetshuffleIndex (+ (Variables|Default|GetshuffleIndex) 1))
    (else
      (Variables|Default|SetshuffleIndex 0))))

(fn ConstructionScript)

(fn SetRandomPresentColor
  (params (ColorArray :type Array%20of%20Linear%20Color%20Structures))
  (bind _output_get (LocalVariables|SetavailableColors ColorArray))
  (bind _output_get_2 (LocalVariables|SetavailableColorsLength (Utilities|Array|Length _output_get)))
  (Development|PrintString (Utilities|String|ToString(Integer) _output_get_2) true true "(R=0.000000,G=0.660000,B=1.000000,A=1.000000)" 1e+02)
  (if (< (LocalVariables|GetavailableColorsLength) 1)
    (Rendering|Material|SetVectorParameterValue "/Game/Presents/presentMainColor.presentMainColor" "presentColor" (Variables|Default|GetdefaultColor) :!class /Script/Engine.KismetMaterialLibrary)
    (else
      (bind _output_get_3 (LocalVariables|SetrandomColor (Utilities|Array|Get(acopy) (LocalVariables|GetavailableColors) (Math|Random|RandomInteger (LocalVariables|GetavailableColorsLength)))))
      (Rendering|Material|SetVectorParameterValue "/Game/Presents/presentMainColor.presentMainColor" "presentColor" _output_get_3 :!class /Script/Engine.KismetMaterialLibrary)
      (Development|PrintString "Present  Color" true true _output_get_3 1e+02)))
  (return (LocalVariables|GetrandomColor)))

(fn SetColorAllowtoChange
  (params (allowChange :type Boolean))
  (Variables|Default|SetallowChange allowChange))

(fn GetAllowChange
  (return (Variables|Default|GetallowChange)))

(fn SwitchColors
  (params (newColor :type Linear%20Color%20Structure))
  (bind _returnvalue (Rendering|Material|GetVectorParameterValue "/Game/Presents/presentMainColor.presentMainColor" "presentColor" :!class /Script/Engine.KismetMaterialLibrary))
  (LocalVariables|SetoldColor _returnvalue)
  (Rendering|Material|SetVectorParameterValue "/Game/Presents/presentMainColor.presentMainColor" "presentColor" newColor :!class /Script/Engine.KismetMaterialLibrary)
  (bind _returnvalue_2 (Actor|GetActorOfClass "/Game/Blueprint/BP_DoorSpawner.BP_DoorSpawner_C"))
  (Default|AddOldtoRemaining _returnvalue_2 (LocalVariables|GetoldColor)))