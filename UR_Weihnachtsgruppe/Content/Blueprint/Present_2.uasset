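; Present_2 is a Blueprint that recolors the present associated with Player 2 after a successful delivery.
; Its delivery-success event passes the available door colors to a function that picks one at random, or uses a default color when none remain.
; The color is written to the PresentColor2 Material Parameter Collection, and a random pick is also printed on screen as debug text.
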(event Custom|Player%202%20Delivery%20on%20success
  (params (available%20door%20colors :type Array%20of%20Linear%20Color%20Structures))
  (CallFunction|SetRandomPresentColor available%20door%20colors))

(event Collision|EventActorBeginOverlap
  (params (OtherActor :type Actor%20Object%20Reference)))

(event EventTick
  (params (DeltaSeconds :type Float%20%28single-precision%29)))

(fn ConstructionScript)

(fn SetRandomPresentColor
  (params (ColorArray :type Array%20of%20Linear%20Color%20Structures))
  (bind _output_get (LocalVariables|SetavalableColors ColorArray))
  (if (== (Utilities|Array|Length _output_get) 0)
    (Rendering|Material|SetVectorParameterValue "/Game/Presents/presentColor2.presentColor2" "presentColor2" (Variables|Default|GetdefaultColor) :!class /Script/Engine.KismetMaterialLibrary)
    (else
      (bind _output_get_2 (LocalVariables|SetrandomColor (Utilities|Array|Get(acopy) (LocalVariables|GetavalableColors) (Math|Random|RandomInteger (Utilities|Array|Length (LocalVariables|GetavalableColors))))))
      (Rendering|Material|SetVectorParameterValue "/Game/Presents/presentColor2.presentColor2" "presentColor2" _output_get_2 :!class /Script/Engine.KismetMaterialLibrary)
      (Development|PrintString "Present  Color" true true _output_get_2 1e+02)))
  (return _output_get_2))