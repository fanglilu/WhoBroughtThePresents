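; Tutorial wrapping-paper pickup that lets a player unlock a color change on their own or the opponent's present.
; Delayed Tick cycles BP_DoorSpawner's GameColors into the ItemPresentColor parameter collection, while box overlaps toggle per-player widgets.
; ActivateWrappingPaper uses DamageOther to pick the present and always calls the timer on BP_Character_Player_1.
; It then removes the widget, spawns ItemCollision_WrappingPaper2 at a random stored transform, plays feedback audio and destroys itself.
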(event OnComponentEndOverlap(Box)
  (params (OverlappedComponent :type Primitive%20Component%20Object%20Reference) (OtherActor :type Actor%20Object%20Reference) (OtherComp :type Primitive%20Component%20Object%20Reference) (OtherBodyIndex :type Integer))
  ;[1 1 1] OnCollisionDetection
  (Variables|Default|SetInTheColliderBox false)
  (if (Variables|Default|GetColliderIsPlayer1)
    (Widget|RemovefromParent (stale OnComponentBeginOverlap(Box) _returnvalue))
    (Variables|Default|SetColliderIsPlayer1 false)
    (Variables|Default|SetWidgetIsActive_Player1 false)
    (elif (Variables|Default|GetColliderIsPlayer2)
      (Widget|RemovefromParent (stale OnComponentBeginOverlap(Box) _returnvalue_2))
      (Variables|Default|SetColliderIsPlayer2 false)
      (Variables|Default|SetWidgetIsActive_Player2 false))))

(event OnComponentBeginOverlap(Box)
  (params (OverlappedComponent :type Primitive%20Component%20Object%20Reference) (OtherActor :type Actor%20Object%20Reference) (OtherComp :type Primitive%20Component%20Object%20Reference) (OtherBodyIndex :type Integer) (bFromSweep :type Boolean) (SweepResult :type Hit%20Result%20Structure%20%28by%20ref%29))
  ;[1 1 1] OnCollisionDetection
  (Variables|Default|SetInTheColliderBox true)
  (if (Utilities|ClassIsChildOf (Utilities|GetClass OtherActor) "/Game/Blueprint/BP_Character_Player_1.BP_Character_Player_1_C")
    (Variables|Default|SetColliderIsPlayer1 true)
    (if (not (Variables|Default|GetWidgetIsActive_Player1))
      (Variables|Default|SetWidgetIsActive_Player1 true)
      (bind _returnvalue (UserInterface|CreateWidget "/Game/Blueprint/TutorialWidgets/Tutorial/TUTORIAL_BP_GameWidget_WrappingPaperItem_Player1_2.TUTORIAL_BP_GameWidget_WrappingPaperItem_Player1_2_C"))
      (UserInterface|Viewport|AddtoViewport _returnvalue 0))
    (elif (Utilities|ClassIsChildOf (Utilities|GetClass OtherActor) "/Game/Blueprint/BP_Character_Player_2.BP_Character_Player_2_C")
      (Variables|Default|SetColliderIsPlayer2 true)
      (if (not (Variables|Default|GetWidgetIsActive_Player2))
        (Variables|Default|SetWidgetIsActive_Player2 true)
        (bind _returnvalue_2 (UserInterface|CreateWidget "/Game/Blueprint/TutorialWidgets/Tutorial/TUTORIAL_BP_GameWidget_WrappingPaperItem_Player2_2.TUTORIAL_BP_GameWidget_WrappingPaperItem_Player2_2_C"))
        (UserInterface|Viewport|AddtoViewport _returnvalue_2 0)))))

(event Custom|ActivateWrappingPaper
  (params (DamageOther :type Boolean))
  (if DamageOther
    (if (and (Variables|Default|GetInTheColliderBox) (Variables|Default|GetColliderIsPlayer1))
      (bind _returnvalue (Actor|GetActorOfClass "/Game/Blueprint/BP_Character_Player_1.BP_Character_Player_1_C"))
      (Default|TriggerTimer _returnvalue true false true false)
      (bind _returnvalue_2 (Actor|GetActorOfClass "/Game/Blueprint/Present_2.Present_2_C"))
      (Default|SetColorAllowtoChange _returnvalue_2 true)
      (if (Variables|Default|GetWidgetIsActive_Player1) :!label _label
        (Widget|RemovefromParent (stale OnComponentBeginOverlap(Box) _returnvalue))
        (Variables|Default|SetWidgetIsActive_Player1 false)
        (Game|SpawnActorfromClass "/Game/Blueprint/ItemCollision_WrappingPaper2.ItemCollision_WrappingPaper2_C" (Utilities|Array|Get(acopy) (Variables|Default|GetTransformArray) (Math|Random|RandomIntegerinRange 0 (- (Utilities|Array|Length (Variables|Default|GetTransformArray)) 1))) "Undefined" 0 0 :!label _label_2)
        (if DamageOther
          (Audio|PlaySound2D "/Game/Music/SoundEffects/mixkit-wrong-answer-fail-notification-946.mixkit-wrong-answer-fail-notification-946" 1.0 1.0 0.0 0 0)
          (else
            (Audio|PlaySound2D "/Game/Music/SoundEffects/mixkit-positive-notification-951.mixkit-positive-notification-951" 1.0 1.0 0.0 0 0)))
        (Actor|DestroyActor)
        (elif (Variables|Default|GetWidgetIsActive_Player2)
          (Widget|RemovefromParent (stale OnComponentBeginOverlap(Box) _returnvalue_2))
          (Variables|Default|SetWidgetIsActive_Player2 false)
          (goto _label_2)))
      (elif (and (Variables|Default|GetInTheColliderBox) (Variables|Default|GetColliderIsPlayer2))
        (bind _returnvalue_3 (Actor|GetActorOfClass "/Game/Blueprint/BP_Character_Player_1.BP_Character_Player_1_C"))
        (Default|TriggerTimer _returnvalue_3 false false true false)
        (bind _returnvalue_4 (Actor|GetActorOfClass "/Game/Blueprint/Present_1.Present_1_C"))
        (Default|SetColorAllowtoChange _returnvalue_4 true)
        (goto _label)))
    (elif (and (Variables|Default|GetInTheColliderBox) (Variables|Default|GetColliderIsPlayer1))
      (bind _returnvalue_5 (Actor|GetActorOfClass "/Game/Blueprint/BP_Character_Player_1.BP_Character_Player_1_C"))
      (Default|TriggerTimer _returnvalue_5 true false true false)
      (bind _returnvalue_6 (Actor|GetActorOfClass "/Game/Blueprint/Present_1.Present_1_C"))
      (Default|SetColorAllowtoChange _returnvalue_6 true)
      (goto _label)
      (elif (and (Variables|Default|GetInTheColliderBox) (Variables|Default|GetColliderIsPlayer2))
        (bind _returnvalue_7 (Actor|GetActorOfClass "/Game/Blueprint/BP_Character_Player_1.BP_Character_Player_1_C"))
        (Default|TriggerTimer _returnvalue_7 false false true false)
        (bind _returnvalue_8 (Actor|GetActorOfClass "/Game/Blueprint/Present_2.Present_2_C"))
        (Default|SetColorAllowtoChange _returnvalue_8 true)
        (goto _label)))))

(event EventTick
  (params (DeltaSeconds :type Float%20%28single-precision%29))
  (Utilities|FlowControl|Delay 0.5)
  (bind _returnvalue (Actor|GetActorOfClass "/Game/Blueprint/BP_DoorSpawner.BP_DoorSpawner_C"))
  (Rendering|Material|SetVectorParameterValue "/Game/Presents/itemPresentColor.itemPresentColor" "itemColor" (Utilities|Array|Get(acopy) (Variables|/Game/Blueprint/BP_DoorSpawner.BP_DoorSpawner_C|GetGameColors _returnvalue) (Variables|Default|GetColorIndex)) :!class /Script/Engine.KismetMaterialLibrary)
  (bind _result (Math|Integer|DecrementInt (Utilities|Array|Length (Variables|/Game/Blueprint/BP_DoorSpawner.BP_DoorSpawner_C|GetGameColors _returnvalue)))
    (:%20%20
      (if (== _result (Variables|Default|GetColorIndex))
        (Variables|Default|SetColorIndex 0)
        (else
          (Math|Integer|IncrementInt (Variables|Default|GetColorIndex)))))))

(fn ConstructionScript)